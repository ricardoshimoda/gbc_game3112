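; BP_PlayerPawn is a player pawn Blueprint prototyping a cover system, though none of its EventGraph logic is connected to run.
; Toggling cover traces along the overlapped box's forward vector and snaps the pawn a capsule radius from the hit.
; In cover, sideways input follows the box's right vector, clamped to its extent by dot-product projection, with debug drawing.
; Forward input is blocked, and mesh rotation depends on cover and aiming.
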(fn `UserConstructionScript`)