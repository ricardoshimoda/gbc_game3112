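; BP_Test_HumanoidAI is a test humanoid AI character that runs the Test_BT_V2 behavior tree.
; On BeginPlay, only on the authority, it starts the tree through its AI controller and binds an OnDeath handler, which is empty.
; Unconnected leftover logic would set the player pawn as blackboard Target and release a claimed CoverSpotV2 while disabling movement avoidance.
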(event `self.ReceiveBeginPlay`
  (if (`|EnumEquality` (`self.GetLocalRole`) "ROLE_Authority")
    (`AIController.RunBehaviorTree` (`AIBlueprintHelperLibrary.GetAIController` self) "/Game/AI/Test_BT_V2.Test_BT_V2")
    (add `self.OnDeath` (delegate `On_Death_Event`))))

(event `On_Death_Event` :!signature `self.OnDeath`
  (params (actor :type "TPSCharacter Object Reference")))

(fn `UserConstructionScript`)