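; Behavior Tree service that finds a cover spot from the player for an AI pawn and writes it to the FoundCoverSpot blackboard key.
; Each tick it sphere-overlaps nearby BP_CoverTemp actors and insertion-sorts them by distance to the player.
; It picks covers with an unblocked trace from above to the player.
; It returns a free or self-used child CoverSpotV2 whose trace to the player hits that cover.
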(event `self.ReceiveTickAI`
  (params (OwnerController :type "AIController Object Reference") (ControlledPawn :type "Pawn Object Reference") (DeltaSeconds :type "Float (single-precision)"))
  (bind (_foundcover _coverspot) (`self.FindCoverSpotOverlap` ControlledPawn))
  (if _foundcover
    (`BTFunctionLibrary.SetBlackboardValueAsObject` (`self.FoundCoverSpot`) _coverspot)))

(fn `FindCoverSpotOverlap`
  (params (Owner :type "Pawn Object Reference"))
  (returns (foundCover :type Boolean) (CoverSpot :type "/Game/BluePrints/CoverSpotV2 Object Reference"))
  (bind _returnvalue (`GameplayStatics.GetPlayerPawn` 0))
  (bind _returnvalue_2 (`GameplayStatics.GetPlayerPawn` 0))
  (bind _coveranddistancearray (`self.CoverAndDistanceArray`))
  (bind _coveranddistancearray_2 (`self.CoverAndDistanceArray`))
  ;[1 1 1] Gets All Cover Spots in a Sphere surrounding the bot
  (bind (_outactors _returnvalue_3) (`KismetSystemLibrary.SphereOverlapActors` (`Actor.K2_GetActorLocation` Owner) (`self.Range`) (`|MakeArray` "ObjectTypeQuery2" :!type "EObjectTypeQuery Enum") "/Game/BluePrints/BP_CoverTemp.BP_CoverTemp_C"))
  ;[1 1 1] Clears the ordering array and calculates the distance for each cover point
  (`KismetArrayLibrary.Array_Clear` (`self.CoverAndDistanceArray`))
  (for _array_element _outactors
    (bind _returnvalue_4 (`KismetMathLibrary.Vector_Distance` (`Actor.K2_GetActorLocation` _array_element) (`Actor.K2_GetActorLocation` (`GameplayStatics.GetPlayerPawn` 0))))
    (bind _output_get (set `self.CurrentActorDistance` (make `/Game/BluePrints/CoverPointAndDistance` _array_element _returnvalue_4)))
    ;[1 1 1] Implements Insert Sort
    (if (== 0 (`KismetArrayLibrary.Array_Length` _coveranddistancearray_2))
      ;[1 1 1] Inserts the first member
      (`KismetArrayLibrary.Array_Insert` _coveranddistancearray_2 _output_get)
      (else
        (for (_array_element_2 _array_index) _coveranddistancearray
          (bind _output_get_2 (set `self.CurrentIndex` _array_index))
          (`/Engine/EditorBlueprintResources/StandardMacros.CompareFloat` (`.DistanceToPlayer_5_99470C4C4E5C7E1919F29C9EBCAED522` (break `/Game/BluePrints/CoverPointAndDistance` _array_element_2)) _returnvalue_4
            (:`>`
              (break))))
        (`KismetArrayLibrary.Array_Insert` _coveranddistancearray _output_get _output_get_2))))
  ;[1 1 1] Recreates the Cover Array - now ordered
  (`KismetArrayLibrary.Array_Clear` (`self.FinalCoverArray`))
  (for (_array_element_3 _array_index_2) (`self.CoverAndDistanceArray`)
    (bind (_coverpoint _distancetoplayer) (break `/Game/BluePrints/CoverPointAndDistance` _array_element_3))
    (`KismetSystemLibrary.PrintString` (`KismetStringLibrary.Conv_DoubleToString` _distancetoplayer))
    (`KismetArrayLibrary.Array_Insert` (`self.FinalCoverArray`) _coverpoint _array_index_2))
  ;[1 1 1] Error Situations - cast and so on
  (if _returnvalue_3
    (for _array_element_4 (`self.FinalCoverArray`)
      ;[1 1 1] Verifies if there is a direct linetrace between the player and the bot in this cover spot - if not then this is a good cover spot
      (bind _asbp_cover_temp (cast `/Game/BluePrints/BP_CoverTemp` _array_element_4)
        (:`then`
          (if (`KismetSystemLibrary.IsValid` _returnvalue_2)
            (bind (_outhit _returnvalue_5) (`KismetSystemLibrary.LineTraceSingle` (+ (`Actor.K2_GetActorLocation` _asbp_cover_temp) (0.0 0.0 200.0)) (`Actor.K2_GetActorLocation` _returnvalue_2) "TraceTypeQuery1" false (`|MakeArray` _returnvalue_2 :!type "Actor Object Reference")))
            (if (not _returnvalue_5)
              ;[1 1 1] Verifies if the cover spot is busy or not - and if its
              (for _array_element_5 (`/Game/BluePrints/BP_CoverTemp.CoverSpots` _asbp_cover_temp)
                (bind _ascover_spot_v2 (cast `/Game/BluePrints/CoverSpotV2` (`ChildActorComponent.ChildActor` _array_element_5)))
                (if (or (`|EnumEquality` (`/Game/BluePrints/CoverSpotV2.CurrentState` _ascover_spot_v2) "NewEnumerator0") (== (`/Game/BluePrints/CoverSpotV2.CurrentUser` _ascover_spot_v2) (`self.ControlledPawn`)))
                  ;[1 1 1] Verifies once more if there is a cover between the player and the selected cover spot
                  (if (`KismetSystemLibrary.IsValid` _returnvalue)
                    (bind (_outhit_2 _returnvalue_6) (`KismetSystemLibrary.LineTraceSingle` (`Actor.K2_GetActorLocation` _ascover_spot_v2) (`Actor.K2_GetActorLocation` _returnvalue) "TraceTypeQuery4"))
                    (if _returnvalue_6
                      (if (== (`.HitActor` (`GameplayStatics.BreakHitResult` _outhit_2)) _asbp_cover_temp)
                        (return true _ascover_spot_v2)))
                    (else
                      (return false null))))))
            (else
              (return false null))))
        (:`CastFailed`
          (return false null))))
    (return false null)
    (else
      (return false null))))